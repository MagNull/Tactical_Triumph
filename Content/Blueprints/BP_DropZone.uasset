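; BP_DropZone is a placement zone that spawns a BP_Hero at its own transform and stores it as its hero.
; SpawnCharacter then registers the zone with the Squad component on the first player's pawn; its CharacterAsset input is unused here.
; ApplyZoneTag marks the new hero through GAS, adding the zone's GrantedTag to a GE_InfiniteEffect spec applied to the hero itself.
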(event `self.ReceiveBeginPlay`)

(fn `ApplyZoneTag`
  (params (Hero :type "Hero Object Reference"))
  (bind _abilitysystemcomponent (`Hero.AbilitySystemComponent` Hero))
  (bind _returnvalue (`AbilitySystemBlueprintLibrary.AddGrantedTag` (`AbilitySystemComponent.MakeOutgoingSpec` :`self` _abilitysystemcomponent :`GameplayEffectClass` "/Game/Blueprints/AbilitySystem/GameplayEffects/GE_InfiniteEffect.GE_InfiniteEffect_C") (`self.GrantedTag`)))
  (`AbilitySystemComponent.BP_ApplyGameplayEffectSpecToSelf` _abilitysystemcomponent _returnvalue))

(fn `SpawnCharacter`
  (params (CharacterAsset :type "DA_Card Object Reference"))
  (bind _returnvalue (`|SpawnActorFromClass` "/Game/Blueprints/BP_Hero.BP_Hero_C" (`self.GetTransform` self) "Undefined" "MultiplyWithRoot" null null))
  (`self.SetHero` _returnvalue)
  (`Squad.AddHero` (`self.GetComponentByClass` (`GameplayStatics.GetPlayerPawn` 0) "/Script/Tactical_Triumph.Squad") self)
  (`self.ApplyZoneTag` _returnvalue))

(fn `UserConstructionScript`)