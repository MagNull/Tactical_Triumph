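; Drop zone where character assets are recruited and heroes are spawned for the active player.
; RecruitCharacter sends a Gameplay Ability System recruit event carrying the asset to the active player, then returns whether the zone is occupied.
; SpawnCharacter creates a BP_Hero at the zone's transform, owned by that player, and registers it with the zone.
; Heroes tagged as Leader lose their first Move-tagged ability on spawn.
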(fn `RecruitCharacter`
  (params (CharacterAsset :type "HeroData Object Reference"))
  (returns (Succed :type Boolean))
  (if (`KismetSystemLibrary.IsValid` CharacterAsset)
    (bind _returnvalue (`BattleState.GetActivePlayer`))
    (`AbilitySystemBlueprintLibrary.SendGameplayEventToActor` _returnvalue (struct :`TagName` "Player.Event.Recruit") (make `GameplayEventData` (struct) self null CharacterAsset))
    (return (`self.IsOccupied`))))

(fn `Spawn Character`
  (params (CharacterAsset :type "HeroData Object Reference"))
  (bind _returnvalue (`BattleState.GetActivePlayer`))
  (bind _returnvalue_2 (`|SpawnActorFromClass` "/Game/Blueprints/BP_Hero.BP_Hero_C" (`self.GetTransform`) "Undefined" "MultiplyWithRoot" null _returnvalue null))
  (`self.SetHero` _returnvalue_2)
  (bind _abilitysystemcomponent (`Hero.AbilitySystemComponent` _returnvalue_2))
  (if (`GameplayTagAssetInterface.HasMatchingGameplayTag` _abilitysystemcomponent (struct :`TagName` "Hero.Position.Leader"))
    (bind _outabilityhandles (`AbilitySystemComponent.FindAllAbilitiesWithTags` _abilitysystemcomponent (struct :`GameplayTags` (struct :`(TagName` "Ability.Type.Move"))) true))
    (`AbilitySystemComponent.ClearAbility` _abilitysystemcomponent (`|GetArrayItem` _outabilityhandles)))
  (return))

(fn `UserConstructionScript`)