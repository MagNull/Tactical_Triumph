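; BP_DropZone is a floor slot where the active player recruits a hero.
; RecruitCharacter spawns a BP_Hero at the zone's transform, initializes it with the character asset and the zone's granted position tag, and stores it as the occupant.
; It then sends a Player.Event.Recruit gameplay event to the player with the asset as payload and returns the occupancy state.
; SetActiveMaterial swaps the mesh material to show whether the zone is active.
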(fn `RecruitCharacter`
  (params (CharacterAsset :type "HeroData Object Reference"))
  (returns (Succed :type Boolean))
  (if (`KismetSystemLibrary.IsValid` CharacterAsset)
    (`self.Spawn Character` CharacterAsset)
    (`AbilitySystemBlueprintLibrary.SendGameplayEventToActor` (`BattleState.GetActivePlayer`) (struct :`TagName` "Player.Event.Recruit") (make `GameplayEventData` (struct) self null CharacterAsset))
    (return (`self.IsOccupied`))))

(fn `SetActiveMaterial`
  (params (IsActive :type Boolean))
  (bind _staticmesh (`self.StaticMesh`))
  (if IsActive
    (`PrimitiveComponent.SetMaterial` _staticmesh 0 "/Engine/EditorMaterials/PersonaFloorMat.PersonaFloorMat")
    (else
      (`PrimitiveComponent.SetMaterial` _staticmesh 0 "/Engine/BasicShapes/BasicShapeMaterial.BasicShapeMaterial"))))

(fn `Spawn Character`
  (params (CharacterAsset :type "HeroData Object Reference"))
  (bind _returnvalue (`|SpawnActorFromClass` "/Game/Blueprints/BP_Hero.BP_Hero_C" (`self.GetTransform`) "Undefined" "MultiplyWithRoot" null (`BattleState.GetActivePlayer`) null))
  (`/Game/Blueprints/BP_Hero.Init` _returnvalue CharacterAsset (`self.GetGrantedTag`))
  (`self.SetHero` _returnvalue)
  (return))

(fn `UserConstructionScript`)