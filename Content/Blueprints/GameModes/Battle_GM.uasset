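; Battle game mode that runs turn order, advancing play through nested turns, waves and rounds.
; On BeginPlay it finds the BP_TurnButton actor, binds to its click and hooks debug prints to the three end events.
; ChangePlayerTurn switches the active player, ending a wave and advancing the line when play returns to the starting player.
; When the line wraps to zero, the round ends, changing the start player and turn count.
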(event `self.ReceiveBeginPlay`
  (bind _returnvalue (`GameplayStatics.GetActorOfClass` "/Game/Blueprints/BP_TurnButton.BP_TurnButton_C"))
  (bind _output_get (set `self.TurnButton` _returnvalue))
  (add `self.OnClicked` _output_get (`|CreateDelegate` :!event `ChangePlayerTurn`))
  (add `self.OnEndTurn` (delegate `OnEndTurn_Event`))
  (add `self.OnEndWave` (delegate `OnEndWave_Event`))
  (add `self.OnEndRound` (delegate `OnEndRound_Event`)))

(event `OnEndTurn_Event`
  (`KismetSystemLibrary.PrintString` "End Turn"))

(event `OnEndWave_Event`
  (`KismetSystemLibrary.PrintString` "End Wave"))

(event `OnEndRound_Event`
  (`KismetSystemLibrary.PrintString` "End Round"))

(fn `ChangePlayerTurn`
  (params (TouchedActor :type "Actor Object Reference") (ButtonPressed :type "Key Structure" :default "None"))
  (`self.OnEndTurn`)
  (`BattleState.ChangeActivePlayer`)
  (bind _returnvalue (`BattleState.GetActivePlayerIndex`))
  (bind _returnvalue_2 (`BattleState.GetStartPlayerIndex`))
  (if (== _returnvalue _returnvalue_2)
    (`self.OnEndWave`)
    (`BattleState.ChangeLineTurn`)
    (bind _returnvalue_3 (`BattleState.GetLineTurnInt`))
    (if (== _returnvalue_3 0)
      (`self.OnEndRound`)
      (`BattleState.ChangeStartPlayerIndex`)
      (`BattleState.AddTurnCount`)
      (`BattleState.ChangeActivePlayer`))))

(fn `UserConstructionScript`)