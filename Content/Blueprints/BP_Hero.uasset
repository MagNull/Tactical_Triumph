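; BP_Hero is a squad hero actor built on the Gameplay Ability System for turn-based play.
; Init uses HeroData and a position tag to set mesh, SetByCaller attributes and abilities, with separate Leader stats.
; Valid clicks on the active player's current row open HeroWidget, whose buttons activate abilities by tag.
; Attribute changes update the widget, death swaps abilities for corpse removal, and debug keys apply damage or print effects.
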(event `Key|MiddleMouseButton`
  (params (Key :type "Key Structure"))
  (:`Pressed`
    (`AbilitySystemComponent.BP_ApplyGameplayEffectToSelf` :`self` (`self.AbilitySystemComponent`) :`GameplayEffectClass` "/Game/Blueprints/AbilitySystem/GameplayEffects/Generic/GE_ApplyDamage.GE_ApplyDamage_C")))

(event `InputConfirmed`
  (`AbilitySystemComponent.TargetConfirm` (`self.AbilitySystemComponent`)))

(event `Key|D`
  (params (Key :type "Key Structure"))
  (:`Pressed`
    (bind _result (`self.Get All Effects Names`)
      (:`Out`
        (`KismetSystemLibrary.PrintString` _result)))))

(event `InputCanceled`
  (`AbilitySystemComponent.TargetCancel` (`self.AbilitySystemComponent`)))

(event `self.ReceiveActorOnClicked`
  (params (ButtonPressed :type "Key Structure"))
  ;[1 1 1] Selection
  (bind _valid (`self.IsValidClick`))
  (if _valid
    (`/Game/Blueprints/BP_HeroWidget.Enable` (`self.Hero Widget`) self)
    (`PrimitiveComponent.SetCollisionEnabled` (`self.Widget`) "QueryAndPhysics")
    (`/Game/Blueprints/BP_Player.ShowDescriptionPanel` (`self.PlayerOwner`) (`self.Hero Data`))))

(event `self.OnAttackChanged`
  (params (deltaValue :type "Float (single-precision)") (eventTags :type "GameplayTagContainer Structure (by ref)"))
  ;[1 1 1] Attribute Changed Events
  (`/Game/Blueprints/BP_HeroWidget.On Attack Changed` (`self.Hero Widget`) (`self.GetAttack`)))

(event `self.OnDamageChanged`
  (params (DamageAmount :type "Float (single-precision)") (DamageTags :type "GameplayTagContainer Structure") (DamageInstigator :type "AbilitySystemComponent Object Reference") (Target :type "AbilitySystemComponent Object Reference"))
  ;[1 1 1] Attribute Changed Events
  (if (> DamageAmount 0.0)
    (`AbilitySystemBlueprintLibrary.SendGameplayEventToActor` self (struct :`TagName` "Hero.Event.Damaged")))
  (`/Game/Blueprints/BP_HeroWidget.On Damage Changed` (`self.Hero Widget`) (`self.GetPresentDamage`)))

(event `self.OnHealthChanged`
  (params (deltaValue :type "Float (single-precision)") (eventTags :type "GameplayTagContainer Structure (by ref)"))
  ;[1 1 1] Attribute Changed Events
  (`/Game/Blueprints/BP_HeroWidget.On Health Changed` (`self.Hero Widget`) (`self.GetHealth`)))

(event `self.Died`
  ;[1 1 1] Died
  (`self.OnDied`))

(event `Init`
  (params (`Hero  Data` :type "HeroData Object Reference") (`Position Tag` :type "GameplayTag Structure"))
  ;[1 1 1] Init Hero
  (set `self.Hero Data` `Hero  Data`)
  (bind _asbp_hero_widget (cast `/Game/Blueprints/BP_HeroWidget` (`WidgetComponent.GetUserWidgetObject` (`self.Widget`))))
  (bind _output_get (set `self.Hero Widget` _asbp_hero_widget))
  (`self.Initialize` `Position Tag`)
  ;[1 1 1] Init Widget
  (`/Game/Blueprints/BP_HeroWidget.Init` _output_get self)
  (`/Game/Blueprints/BP_HeroWidget.Deactivate` _output_get)
  (`PrimitiveComponent.SetCollisionEnabled` (`self.Widget`) "NoCollision")
  (add `/Game/Blueprints/BP_HeroWidget.Clicked` (`self.Hero Widget`) (delegate `WidgetButtonClicked`)))

(event `WidgetButtonClicked`
  (params (`Clicked Action Tag` :type "GameplayTagContainer Structure"))
  ;[1 1 1] Init Widget
  (`AbilitySystemComponent.TryActivateAbilitiesByTag` (`self.AbilitySystemComponent`) `Clicked Action Tag` true)
  (`PrimitiveComponent.SetCollisionEnabled` (`self.Widget`) "NoCollision"))

(event `self.ReceiveDestroyed`
  ;[1 1 1] Init Widget
  (clear `/Game/Blueprints/BP_HeroWidget.Clicked` (`self.Hero Widget`)))

(fn `ApplyDefaultAttributeValue`
  (params (Attack :type "Float (double-precision)") (Health :type "Float (double-precision)"))
  (bind _returnvalue (`AbilitySystemBlueprintLibrary.AssignTagSetByCallerMagnitude` (`AbilitySystemComponent.MakeOutgoingSpec` :`self` (`self.AbilitySystemComponent`) :`GameplayEffectClass` "/Game/Blueprints/AbilitySystem/GameplayEffects/Generic/GE_SetDefaultAttributesValue.GE_SetDefaultAttributesValue_C" :`Level` 1.0) (struct :`TagName` "Hero.Attribute.MaxHealth") Health))
  (bind _returnvalue_2 (`AbilitySystemBlueprintLibrary.AssignTagSetByCallerMagnitude` _returnvalue (struct :`TagName` "Hero.Attribute.Health") Health))
  (bind _returnvalue_3 (`AbilitySystemBlueprintLibrary.AssignTagSetByCallerMagnitude` _returnvalue_2 (struct :`TagName` "Hero.Attribute.Attack") Attack))
  (`AbilitySystemComponent.BP_ApplyGameplayEffectSpecToSelf` (`self.AbilitySystemComponent`) _returnvalue_3))

(fn `ApplySkeletalMesh`
  (`/Engine/EditorBlueprintResources/StandardMacros.IsValid` (`self.Hero Data`)
    (:`Is Valid`
      (`SkeletalMeshComponent.SetSkeletalMeshAsset` (`self.Mesh`) (`/Game/Blueprints/BP_HeroData.Mesh` (`self.Hero Data`))))
    (:`Is Not Valid`
      (`SkeletalMeshComponent.SetSkeletalMeshAsset` (`self.Mesh`) "/Engine/EngineMeshes/SkeletalCube.SkeletalCube"))))

(fn `Can Activate Ability with Tag`
  (params (Tag :type "GameplayTagContainer Structure"))
  (returns (Can :type Boolean))
  (bind _returnvalue (`HeroAbilitySystemComponent.CanActivateAbilityWithTag` (`self.AbilitySystemComponent`) Tag))
  (return _returnvalue))

(fn `GrantDefaultAbilities`
  (params (`Position Tag` :type "GameplayTag Structure"))
  (bind _ashero_ability_system_component (cast `HeroAbilitySystemComponent` (`AbilitySystemBlueprintLibrary.GetAbilitySystemComponent` null)))
  (`HeroAbilitySystemComponent.SetAbilitySquadLineMap` _ashero_ability_system_component (`/Game/Blueprints/BP_HeroData.Abilities` (`self.Hero Data`)))
  (`AbilitySystemComponent.K2_GiveAbility` (`self.AbilitySystemComponent`) null 0 -1)
  (if (!= `Position Tag` (struct :`TagName` "Hero.Position.Leader"))
    (`AbilitySystemComponent.K2_GiveAbility` (`self.AbilitySystemComponent`) "/Game/Blueprints/AbilitySystem/GameplayAbilities/GA_HeroMove.GA_HeroMove_C" 0 -1)))

(fn `Initialize`
  (params (`Position Tag` :type "GameplayTag Structure"))
  (locals (`New Post Tag` :type "GameplayTag Structure"))
  (bind _hero_data (`self.Hero Data`))
  (bind _hero_data_2 (`self.Hero Data`))
  (bind _output_get (set `local.New Post Tag` `Position Tag`))
  (`self.ApplySkeletalMesh`)
  (if (== _output_get (struct :`TagName` "Hero.Position.Leader"))
    (`self.ApplyDefaultAttributeValue` (`HeroData.LeaderAttack` _hero_data_2) (`HeroData.LeaderHealth` _hero_data_2))
    (else
      (`self.ApplyDefaultAttributeValue` (`HeroData.Attack` _hero_data) (`HeroData.Health` _hero_data))))
  (`self.GrantDefaultAbilities` (`local.New Post Tag`))
  (bind _returnvalue (`GameplayStatics.GetActorOfClass` "/Game/Blueprints/BP_InputReciever.BP_InputReciever_C"))
  (`/Engine/EditorBlueprintResources/StandardMacros.IsValid` _returnvalue
    (:`Is Valid`
      (add `/Game/Blueprints/BP_InputReciever.Confirm` _returnvalue (`|CreateDelegate` :!event `InputConfirmed`))
      (add `/Game/Blueprints/BP_InputReciever.Cancel` _returnvalue (`|CreateDelegate` :!event `InputCanceled`))
      (`SceneComponent.K2_SetWorldRotation` (`self.Widget`) (struct :`Pitch` 45.0 :`Yaw` 180.0) false false))
    (:`Is Not Valid`
      (`KismetSystemLibrary.PrintString` "Input Reciever is not valid" true true (struct :`R` 1.0 :`A` 1.0)))))

(fn `IsValidClick`
  (returns (Valid :type Boolean))
  (bind _returnvalue (`BattleState.GetLineTurnInt`))
  (return (and (== (`BattleState.GetActivePlayer`) (`self.PlayerOwner`)) (== _returnvalue (`DropZone.GetRowInt` (`SquadComponent.GetDropZoneByHero` (`self.GetComponentByClass` (`BattleState.GetActivePlayer`) "/Script/Tactical_Triumph.SquadComponent") self))))))

(fn `OnDied`
  (bind _abilitysystemcomponent (`self.AbilitySystemComponent`))
  (`AbilitySystemComponent.ClearAllAbilities` (`self.AbilitySystemComponent`))
  (bind _returnvalue (`AbilitySystemBlueprintLibrary.AddGrantedTag` (`AbilitySystemComponent.MakeOutgoingSpec` :`self` (`self.AbilitySystemComponent`)) (struct :`TagName` "Hero.Status.Died")))
  (`AbilitySystemComponent.BP_ApplyGameplayEffectSpecToSelf` _abilitysystemcomponent _returnvalue)
  (`AbilitySystemComponent.K2_GiveAbility` _abilitysystemcomponent "/Game/Blueprints/AbilitySystem/GameplayAbilities/GA_HeroRemoveCorpse.GA_HeroRemoveCorpse_C" 0 -1))

(fn `UserConstructionScript`
  (`self.ApplySkeletalMesh`))