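; GA_PlayerRecruitHero is a player gameplay ability that recruits a hero onto a drop zone when triggered by a gameplay event.
; It commits, requires a BP_DropZone instigator, and spawns a BP_Hero at the zone's transform owned by the active player.
; The hero is initialized with HeroData from the event's optional object and the zone's granted tag, then assigned to that zone.
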(event `self.K2_ActivateAbilityFromEvent`
  (params (EventData :type "GameplayEventData Structure (by ref)"))
  (bind (_eventtag _instigator _target _optionalobject) (break `GameplayEventData` EventData))
  (`self.K2_CommitAbility`)
  (bind _asbp_drop_zone (cast `/Game/Blueprints/DropZone/BP_DropZone` _instigator)
    (:`then`
      (bind _returnvalue (`|SpawnActorFromClass` "/Game/Blueprints/BP_Hero.BP_Hero_C" (`Actor.GetTransform` _asbp_drop_zone) "Undefined" "MultiplyWithRoot" null (`BattleState.GetActivePlayer`) null))
      (bind _ashero_data (cast `HeroData` _optionalobject))
      (`/Game/Blueprints/BP_Hero.Init` _returnvalue _ashero_data (`DropZone.GetGrantedTag` _asbp_drop_zone))
      (`DropZone.SetHero` _asbp_drop_zone _returnvalue))
    (:`CastFailed`
      (`KismetSystemLibrary.PrintString` "Event Recieved not from Drop Zone(Recruit Hero)" true true (struct :`R` 1.0 :`A` 1.0))))
  (`self.K2_EndAbility`))