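; GA_DrawCard is an event-triggered player gameplay ability that draws a card from the owning actor's DeckComponent into its HandleComponent.
; When the deck has cards, it commits the ability cost without checking the result, then pops and adds the card.
; The event's OptionalObject carries W_PlayerUI, which gets a new card widget and count update.
; An invalid pop prints "Deck is Empty" without ending the ability, while an empty deck ends it silently.
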(event `self.K2_ActivateAbilityFromEvent`
  (params (EventData :type "GameplayEventData Structure (by ref)"))
  (bind _returnvalue (`self.GetOwningActorFromActorInfo`))
  (bind _returnvalue_2 (`Actor.GetComponentByClass` _returnvalue "/Script/Tactical_Triumph.DeckComponent"))
  (if (> (`DeckComponent.GetCount` _returnvalue_2) 0)
    (`self.K2_CommitAbilityCost` true)
    (bind _returnvalue_3 (`DeckComponent.Pop` _returnvalue_2))
    (`/Engine/EditorBlueprintResources/StandardMacros.IsValid` _returnvalue_3
      (:`Is Valid`
        (`HandleComponent.AddCard` (`Actor.GetComponentByClass` _returnvalue "/Script/Tactical_Triumph.HandleComponent") _returnvalue_3)
        (bind _asw_player_ui (cast `/Game/Blueprints/Widgets/W_PlayerUI` (`.OptionalObject` (break `GameplayEventData` EventData)))
          (:`then`
            (`/Game/Blueprints/Widgets/W_Handle.AddCardWidget` (`/Game/Blueprints/Widgets/W_PlayerUI.W_Handle` _asw_player_ui) _returnvalue_3)
            (`/Game/Blueprints/Widgets/W_PlayerUI.Update Card Count` _asw_player_ui))
          (:`CastFailed`
            _))
        (`self.K2_EndAbility`))
      (:`Is Not Valid`
        (`KismetSystemLibrary.PrintString` "Deck is Empty" true true (struct :`R` 1.0 :`G` 0.899263 :`A` 1.0))))
    (else
      (`self.K2_EndAbility`))))