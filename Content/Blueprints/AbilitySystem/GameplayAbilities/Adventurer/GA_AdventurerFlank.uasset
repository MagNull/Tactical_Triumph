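; Adventurer Flank gameplay ability that adds attack to the squad zones directly forward of and behind the owning hero.
; On activation it caches both neighbour zones from the squad component and applies GE_AddAttack with a set-by-caller magnitude of round count modulo two.
; It then binds to the battle game mode's round-end event, adding one more attack to both zones whenever the count is even.
; The binding outlives EndAbility and is released on ability removal.
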(event `self.K2_ActivateAbility`
  (`self.Init Neighbours`)
  (bind _returnvalue (`AbilitySystemBlueprintLibrary.AssignTagSetByCallerMagnitude` (`self.MakeOutgoingGameplayEffectSpec` "/Game/Blueprints/AbilitySystem/GameplayEffects/Generic/GE_AddAttack.GE_AddAttack_C") (struct :`TagName` "Ability.Effect.Data.Attack") (`KismetMathLibrary.Conv_Int64ToDouble` (`.ReturnValue` (`KismetMathLibrary.FMod64` (`KismetMathLibrary.Conv_IntToDouble` (`BattleState.GetRoundCount`)) 2.0)))))
  (`DropZone.AddZoneEffect` (`self.Forward Zone`) _returnvalue self)
  (`DropZone.AddZoneEffect` (`self.Back Zone`) _returnvalue self)
  (bind _asbattle_gm (cast `/Game/Blueprints/GameModes/Battle_GM` (`GameplayStatics.GetGameMode`)))
  (add `/Game/Blueprints/GameModes/Battle_GM.OnEndRound` _asbattle_gm (delegate `OnRoundEnd`))
  (`self.K2_EndAbility`))

(event `OnRoundEnd`
  (`self.On Round End`))

(event `self.OnAbilityRemoved`
  (bind _asbattle_gm (cast `/Game/Blueprints/GameModes/Battle_GM` (`GameplayStatics.GetGameMode`)))
  (remove `/Game/Blueprints/GameModes/Battle_GM.OnEndRound` _asbattle_gm (delegate `OnRoundEnd`)))

(fn `Init Neighbours`
  (bind _asbp_hero (cast `/Game/Blueprints/BP_Hero` (`self.GetOwningActorFromActorInfo`)))
  (bind _squadcomponent (`PlayerPawn.SquadComponent` (`/Game/Blueprints/BP_Hero.PlayerOwner` _asbp_hero)))
  (bind _returnvalue (`SquadComponent.GetForwardNeighbour` _squadcomponent _asbp_hero))
  (set `self.Forward Zone` _returnvalue)
  (bind _returnvalue_2 (`SquadComponent.GetBackNeighbour` _squadcomponent _asbp_hero))
  (set `self.Back Zone` _returnvalue_2))

(fn `On Round End`
  (if (== (mod (`BattleState.GetRoundCount`) 2) 0)
    (bind _returnvalue (`AbilitySystemBlueprintLibrary.AssignTagSetByCallerMagnitude` (`self.MakeOutgoingGameplayEffectSpec` "/Game/Blueprints/AbilitySystem/GameplayEffects/Generic/GE_AddAttack.GE_AddAttack_C") (struct :`TagName` "Ability.Effect.Data.Attack") 1.0))
    (`DropZone.AddZoneEffect` (`self.Forward Zone`) _returnvalue self)
    (`DropZone.AddZoneEffect` (`self.Back Zone`) _returnvalue self)))