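; Gameplay ability for the Adventurer Vanguard that grants Attack which grows as battle rounds pass.
; On activation it applies GE_AddAttack to its owner with a set-by-caller magnitude equal to the current round count, binds to the Battle_GM end-round event, then ends.
; The binding outlives the activation, adding one Attack at each round end until the ability is removed and unbinds.
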(event `self.K2_ActivateAbility`
  (bind _returnvalue (`AbilitySystemBlueprintLibrary.AssignTagSetByCallerMagnitude` (`self.MakeOutgoingGameplayEffectSpec` "/Game/Blueprints/AbilitySystem/GameplayEffects/Generic/GE_AddAttack.GE_AddAttack_C") (struct :`TagName` "Ability.Effect.Data.Attack") (`KismetMathLibrary.Conv_IntToDouble` (`BattleState.GetRoundCount`))))
  (`self.K2_ApplyGameplayEffectSpecToOwner` _returnvalue)
  (bind _asbattle_gm (cast `/Game/Blueprints/GameModes/Battle_GM` (`GameplayStatics.GetGameMode`)))
  (add `/Game/Blueprints/GameModes/Battle_GM.OnEndRound` _asbattle_gm (delegate `OnRoundEnd`))
  (`self.K2_EndAbility`))

(event `OnRoundEnd`
  (`self.On Round End`))

(event `self.OnAbilityRemoved`
  (bind _asbattle_gm (cast `/Game/Blueprints/GameModes/Battle_GM` (`GameplayStatics.GetGameMode`)))
  (remove `/Game/Blueprints/GameModes/Battle_GM.OnEndRound` _asbattle_gm (delegate `OnRoundEnd`)))

(fn `On Round End`
  (bind _returnvalue (`AbilitySystemBlueprintLibrary.AssignTagSetByCallerMagnitude` (`self.MakeOutgoingGameplayEffectSpec` "/Game/Blueprints/AbilitySystem/GameplayEffects/Generic/GE_AddAttack.GE_AddAttack_C") (struct :`TagName` "Ability.Effect.Data.Attack") 1.0))
  (`self.K2_ApplyGameplayEffectSpecToOwner` _returnvalue))