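; Gameplay ability for the Adventurer Leader that adds an attack effect to its owner's squad when a round ends.
; On activation it binds to the Battle_GM end-of-round event and ends immediately, leaving the round-end handler to do the work.
; The handler builds a GE_AddAttack spec with a SetByCaller attack magnitude and passes it to the hero's player-owned SquadComponent as a squad effect.
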(event `self.K2_ActivateAbility`
  (bind _asbattle_gm (cast `/Game/Blueprints/GameModes/Battle_GM` (`GameplayStatics.GetGameMode`))
    (:`then`
      (add `/Game/Blueprints/GameModes/Battle_GM.OnEndRound` _asbattle_gm (`|CreateDelegate` :!event `OnRoundEnd`))
      (`self.K2_EndAbility`))
    (:`CastFailed`
      (`KismetSystemLibrary.PrintString` "Adventurer Leader" true true (struct :`R` 1.0 :`B` 0.172167 :`A` 1.0)))))

(fn `OnRoundEnd`
  (locals (NewLocalVar :type "SquadEffect Structure"))
  (`KismetSystemLibrary.PrintString` "Round end" true true (struct :`G` 1.0 :`B` 0.014054 :`A` 1.0))
  (bind _asbp_hero (cast `/Game/Blueprints/BP_Hero` (`self.GetOwningActorFromActorInfo`)))
  (bind _returnvalue (`AbilitySystemBlueprintLibrary.AssignTagSetByCallerMagnitude` (`self.MakeOutgoingGameplayEffectSpec` "/Game/Blueprints/AbilitySystem/GameplayEffects/Generic/GE_AddAttack.GE_AddAttack_C") (struct :`TagName` "Ability.Effect.Data.Attack") 1.0))
  (`SquadComponent.AddSquadEffect` (`PlayerPawn.SquadComponent` (`/Game/Blueprints/BP_Hero.PlayerOwner` _asbp_hero)) (`self.GetSquadEffect` _returnvalue)))