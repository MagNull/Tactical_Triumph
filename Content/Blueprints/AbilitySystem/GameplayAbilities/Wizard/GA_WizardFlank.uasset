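; GA_WizardFlank is a wizard gameplay ability that grants a range attack to the hero and its forward squad neighbour.
; On activation it applies GE_GrantRangeAttack to the owner, then casts the owning actor to Hero.
; It finds the forward neighbour through the active player's SquadComponent and hands it the same effect as a zone effect sourced from this ability.
; The ability then ends, printing a failure message if the cast fails.
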(event `self.K2_ActivateAbility`
  (`self.BP_ApplyGameplayEffectToOwner` "/Game/Blueprints/AbilitySystem/GameplayEffects/Generic/GE_GrantRangeAttack.GE_GrantRangeAttack_C")
  (bind _ashero (cast `Hero` (`self.GetOwningActorFromActorInfo`))
    (:`then`
      (bind _returnvalue (`SquadComponent.GetForwardNeighbour` (`PlayerPawn.SquadComponent` (`BattleState.GetActivePlayer`)) _ashero))
      (`DropZone.AddZoneEffect` _returnvalue (`self.MakeOutgoingGameplayEffectSpec` "/Game/Blueprints/AbilitySystem/GameplayEffects/Generic/GE_GrantRangeAttack.GE_GrantRangeAttack_C") self)
      (`self.K2_EndAbility`))
    (:`CastFailed`
      (`KismetSystemLibrary.PrintString` "Wizard Flank failed" true true (struct :`R` 1.0 :`A` 1.0))
      (`self.K2_EndAbility`))))