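; Wizard Vanguard gameplay ability that damages enemy front-line heroes when its owner is in the front line.
; On activation it commits the cost, then checks whether the owning Hero is among the active player's first heroes in columns.
; If so, it applies a GE_InflictDamage spec, with damage set by caller through a data tag, to each first-in-column hero of the non-active player.
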(event `self.K2_ActivateAbility`
  (`self.K2_CommitAbilityCost` true)
  (bind _ashero (cast `Hero` (`self.GetOwningActorFromActorInfo`)))
  (if (`KismetArrayLibrary.Array_Contains` (`SquadComponent.GetFirstHeroesInColumns` (`PlayerPawn.SquadComponent` (`BattleState.GetActivePlayer`))) _ashero)
    (for _array_element (`SquadComponent.GetFirstHeroesInColumns` (`PlayerPawn.SquadComponent` (`BattleState.GetNotActivePlayer`)))
      (bind _returnvalue (`AbilitySystemBlueprintLibrary.AssignTagSetByCallerMagnitude` (`self.MakeOutgoingGameplayEffectSpec` "/Game/Blueprints/AbilitySystem/GameplayEffects/Generic/GE_InflictDamage.GE_InflictDamage_C") (struct :`TagName` "Ability.Effect.Data.Damage") 3.0))
      (`self.K2_ApplyGameplayEffectSpecToTarget` _returnvalue (`AbilitySystemBlueprintLibrary.AbilityTargetDataFromActor` _array_element)))
    (`self.K2_EndAbility`)
    (else
      (`self.K2_EndAbility`))))