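; Wizard leader gameplay ability that grants its owner a ranged attack and gives the owning player's squad a role-dependent buff.
; On activation and on each Battle_GM round end, it removes its previous squad effect and adds a new one through the SquadComponent.
; The squad gets bonus attack if its player is the attacker, otherwise damage reduction, with magnitudes passed via SetByCaller tags.
; The round-end binding outlives EndAbility and is cleared when the ability is removed.
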(event `self.K2_ActivateAbility`
  (`self.BP_ApplyGameplayEffectToOwner` "/Game/Blueprints/AbilitySystem/GameplayEffects/Generic/GE_GrantRangeAttack.GE_GrantRangeAttack_C")
  (`self.OnRoundEnd`)
  (bind _asbattle_gm (cast `/Game/Blueprints/GameModes/Battle_GM` (`GameplayStatics.GetGameMode`)))
  (add `/Game/Blueprints/GameModes/Battle_GM.OnEndRound` _asbattle_gm (delegate `On Round End`))
  (`self.K2_EndAbility`))

(event `On Round End`
  (`self.OnRoundEnd`))

(event `self.OnAbilityRemoved`
  (bind _asbattle_gm (cast `/Game/Blueprints/GameModes/Battle_GM` (`GameplayStatics.GetGameMode`)))
  (remove `/Game/Blueprints/GameModes/Battle_GM.OnEndRound` _asbattle_gm (delegate `On Round End`)))

(fn `OnRoundEnd`
  (bind _asbp_hero (cast `/Game/Blueprints/BP_Hero` (`self.GetOwningActorFromActorInfo`)))
  (bind _playerowner (`/Game/Blueprints/BP_Hero.PlayerOwner` _asbp_hero))
  (bind _squadcomponent (`PlayerPawn.SquadComponent` _playerowner))
  (`SquadComponent.RemoveSquadEffect` _squadcomponent (`GameplayStatics.GetObjectClass` self))
  (if (== _playerowner (`BattleState.GetAttackPlayer`))
    (bind _returnvalue (`AbilitySystemBlueprintLibrary.AssignTagSetByCallerMagnitude` (`self.MakeOutgoingGameplayEffectSpec` "/Game/Blueprints/AbilitySystem/GameplayEffects/Generic/GE_AddAttack.GE_AddAttack_C") (struct :`TagName` "Ability.Effect.Data.Attack") 2.0))
    (`SquadComponent.AddSquadEffect` _squadcomponent (`self.GetSquadEffect` _returnvalue))
    (else
      (bind _returnvalue_2 (`AbilitySystemBlueprintLibrary.AssignTagSetByCallerMagnitude` (`self.MakeOutgoingGameplayEffectSpec` "/Game/Blueprints/AbilitySystem/GameplayEffects/Generic/GE_AddDamageReduction.GE_AddDamageReduction_C") (struct :`TagName` "Ability.Effect.Data.AttackDamageReduction") 1.0))
      (`SquadComponent.AddSquadEffect` _squadcomponent (`self.GetSquadEffect` _returnvalue_2)))))