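; Gameplay ability that lets a hero move to an empty drop zone in its squad.
; On activation it waits for a user-confirmed target, filtered to the owner's empty drop zones, and highlights the active player's empty zones.
; A valid pick commits the cost and asks the active player's SquadComponent to move the hero to that row and column.
; Ending the ability clears highlights and ends the targeting task.
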(event `self.K2_ActivateAbility`
  (bind _asbp_hero (cast `/Game/Blueprints/BP_Hero` (`self.GetOwningActorFromActorInfo`)))
  (bind _returnvalue (`HeroAbilitiesFunctionLibrary.MakeSelectedFilterHandle` (make `SelectedTargetsFilter` (`SquadComponent.GetEmptyDropZones` (`PlayerPawn.SquadComponent` (`/Game/Blueprints/BP_Hero.PlayerOwner` _asbp_hero))) "/Game/Blueprints/DropZone/BP_DropZone.BP_DropZone_C")))
  (bind (_asynctaskproxy _data) (`AbilityTask_WaitTargetData.WaitTargetData` "None" "UserConfirmed" "/Game/Blueprints/AbilitySystem/GameplayAbilities/Target.Target_C" "Cell" 999999.0 (struct :`Name` "BlockAll") false (struct) (struct) null _returnvalue)
    (:`then`
      (set `self.Async Task` _asynctaskproxy)
      (`self.Highlight Targetable Heroes` _returnvalue))
    (:`ValidData`
      (`self.K2_CommitAbilityCost` true)
      (bind _asdrop_zone (cast `DropZone` (`|GetArrayItem` (`AbilitySystemBlueprintLibrary.GetAllActorsFromTargetData` _data)))
        (:`then`
          (bind _ashero (cast `Hero` (`self.GetOwningActorFromActorInfo`)))
          (`SquadComponent.TryMoveHeroTo` (`Actor.GetComponentByClass` (`BattleState.GetActivePlayer`) "/Script/Tactical_Triumph.SquadComponent") _ashero (`DropZone.Row` _asdrop_zone) (`DropZone.Column` _asdrop_zone)))
        (:`CastFailed`
          (`KismetSystemLibrary.PrintString` "Target of move is not drop zone" true true (struct :`R` 1.0 :`B` 0.018237 :`A` 1.0))))
      (`self.K2_EndAbility` :!label _label))
    (:`Cancelled`
      (goto _label))))

(event `self.K2_OnEndAbility`
  (params (bWasCancelled :type Boolean))
  (bind _target_drop_zones (`self.Target Drop Zones`))
  (bind _async_task (`self.Async Task`))
  (for _array_element _target_drop_zones
    (`/Game/Blueprints/DropZone/BP_DropZone.Disable Highlight` _array_element))
  (`KismetArrayLibrary.Array_Clear` _target_drop_zones)
  (`/Engine/EditorBlueprintResources/StandardMacros.IsValid` _async_task
    (:`Is Valid`
      (`GameplayTask.EndTask` _async_task))))

(fn `Highlight Targetable Heroes`
  (params (Filter :type "GameplayTargetDataFilterHandle Structure"))
  (for _array_element (`SquadComponent.GetEmptyDropZones` (`PlayerPawn.SquadComponent` (`BattleState.GetActivePlayer`)))
    (bind _asbp_drop_zone (cast `/Game/Blueprints/DropZone/BP_DropZone` _array_element))
    (`KismetArrayLibrary.Array_Add` (`self.Target Drop Zones`) _asbp_drop_zone)
    (`/Game/Blueprints/DropZone/BP_DropZone.Highlight` _asbp_drop_zone)))