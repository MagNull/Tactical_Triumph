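; GA_AssasinFlank is the Assassin's Flank gameplay ability, which applies an attack multiplier effect through the owning hero's forward neighbour.
; On activation it asks the active player's SquadComponent for the neighbour in front of the owner.
; It builds a BP_MultiplyAttack spec with a set-by-caller doubling magnitude and adds it to that neighbour as a zone effect.
; The ability ends immediately, printing an error if the owner is not a Hero.
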(event `self.K2_ActivateAbility`
  (bind _ashero (cast `Hero` (`.OwnerActor` (break `GameplayAbilityActorInfo` (`self.GetActorInfo`))))
    (:`then`
      (bind _returnvalue (`SquadComponent.GetForwardNeighbour` (`Actor.GetComponentByClass` (`BattleState.GetActivePlayer`) "/Script/Tactical_Triumph.SquadComponent") _ashero))
      (bind _returnvalue_2 (`AbilitySystemBlueprintLibrary.AssignTagSetByCallerMagnitude` (`self.MakeOutgoingGameplayEffectSpec` "/Game/Blueprints/AbilitySystem/GameplayEffects/Generic/BP_MultiplyAttack.BP_MultiplyAttack_C") (struct :`TagName` "Ability.Effect.Data.Attack") 2.0))
      (`DropZone.AddZoneEffect` _returnvalue _returnvalue_2 self))
    (:`CastFailed`
      (`KismetSystemLibrary.PrintString` "Assasing Flank Cast Error" true true (struct :`R` 1.0 :`G` 0.024519 :`A` 1.0))))
  (`self.K2_EndAbility`))