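; Assassin Vanguard gameplay ability that reacts to the owner's attacks landing on a target tagged as a Leader-position hero.
; It waits for an attack ability to activate, then for an effect applied to such a target, and applies attack damage to that target.
; It then ends, cleaning up both wait tasks, and reactivates its own class to keep listening.
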(event `self.K2_ActivateAbility`
  (bind _asynctaskproxy (`AbilityTask_WaitAbilityActivate.WaitForAbilityActivate` (struct :`TagName` "Ability.Type.Attack") (struct) true)
    (:`then`
      (set `self.Wait Activate` _asynctaskproxy))
    (:`OnActivate`
      (bind (_asynctaskproxy_2 _target) (`AbilityTask_WaitGameplayEffectApplied_Target.WaitGameplayEffectAppliedToTarget` (struct) (struct) (make `GameplayTagRequirements` (struct :`GameplayTags` (struct :`(TagName` "Hero.Position.Leader")))) false null)
        (:`then`
          (set `self.Wait Effect` _asynctaskproxy_2))
        (:`OnApplied`
          (`self.BP_ApplyGameplayEffectToTarget` (`AbilitySystemBlueprintLibrary.AbilityTargetDataFromActor` _target) "/Game/Blueprints/AbilitySystem/GameplayEffects/Generic/GE_AttackDamage.GE_AttackDamage_C")
          (`self.K2_EndAbility`)
          (`AbilitySystemComponent.TryActivateAbilityByClass` (`.AbilitySystemComponent` (break `GameplayAbilityActorInfo` (`self.GetActorInfo`))) "GA_AssasinVanguard_C" true))))))

(event `self.K2_OnEndAbility`
  (params (bWasCancelled :type Boolean))
  (bind _wait_activate (`self.Wait Activate`))
  (bind _wait_effect (`self.Wait Effect`))
  (`/Engine/EditorBlueprintResources/StandardMacros.IsValid` _wait_effect
    (:`Is Valid`
      (`GameplayTask.EndTask` _wait_effect))
    (:`Is Not Valid`
      _))
  (`/Engine/EditorBlueprintResources/StandardMacros.IsValid` _wait_activate
    (:`Is Valid`
      (`GameplayTask.EndTask` _wait_activate))))