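; BP_DropZone is a drop zone that spawns a hero at its own transform and tags it with the zone's position.
; SpawnCharacter spawns a BP_Hero from a valid character data asset, applies the position tag and stores the hero reference.
; ApplyPositionTag uses the Gameplay Ability System, adding the zone's GrantedTag to a GE_InfiniteEffect spec that the hero applies to itself.
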(event `self.ReceiveBeginPlay`)

(fn `ApplyPositionTag`
  (params (`Target Hero` :type "Actor Object Reference"))
  (bind _returnvalue (`AbilitySystemBlueprintLibrary.GetAbilitySystemComponent` `Target Hero`))
  (bind _returnvalue_2 (`AbilitySystemBlueprintLibrary.AddGrantedTag` (`AbilitySystemComponent.MakeOutgoingSpec` :`self` _returnvalue :`GameplayEffectClass` "/Game/Blueprints/AbilitySystem/GameplayEffects/GE_InfiniteEffect.GE_InfiniteEffect_C") (`self.GrantedTag`)))
  (`AbilitySystemComponent.BP_ApplyGameplayEffectSpecToSelf` _returnvalue _returnvalue_2))

(fn `SpawnCharacter`
  (params (CharacterAsset :type "HeroData Object Reference"))
  (if (`KismetSystemLibrary.IsValid` CharacterAsset)
    (bind _returnvalue (`|SpawnActorFromClass` "/Game/Blueprints/BP_Hero.BP_Hero_C" (`self.GetTransform` self) "Undefined" "MultiplyWithRoot" null CharacterAsset null))
    (`self.ApplyPositionTag` _returnvalue)
    (`self.SetHero` _returnvalue)
    (else
      (`KismetSystemLibrary.PrintString` "Failed cast to BP_HeroData"))))

(fn `UserConstructionScript`)