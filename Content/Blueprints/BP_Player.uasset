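; BP_Player is a participant in a turn-based card battle, using the Gameplay Ability System for action points and abilities.
; On start it grants remove-corpse and recruit-hero abilities, sets action points through a set-by-caller effect, and binds to Battle_GM events.
; Turn end restores points if it is the active player; wave end applies damage effects to squad heroes.
; It also toggles drop-zone highlights and a card description panel.
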(event `Key|A`
  (params (Key :type "Key Structure"))
  (:`Pressed`
    (`KismetSystemLibrary.PrintString` (`KismetStringLibrary.BuildString_Int` "Action Points of " (`KismetSystemLibrary.GetDisplayName` (`BattleState.GetActivePlayer`)) (`self.GetActionPoints`)))))

(event `self.ReceiveBeginPlay`
  (`self.Initialize`))

(event `self.OnActionPointsChanged`
  (params (NewValue :type Integer))
  (`self.Action Points Changed` NewValue)
  (`KismetSystemLibrary.PrintString` (`KismetStringLibrary.BuildString_Int` (`KismetSystemLibrary.GetDisplayName` self) "Points changed: " (`self.GetActionPoints`))))

(fn `HideDescriptionPanel`
  (`/Game/Blueprints/Widgets/W_CardDescription.Set Active` (`self.CardDescriptionPanel`) false null false))

(fn `Initialize`
  (bind _abilitysystemcomponent (`self.AbilitySystemComponent`))
  (`AbilitySystemComponent.K2_GiveAbility` _abilitysystemcomponent "/Game/Blueprints/AbilitySystem/GameplayAbilities/Player/GA_PlayerRemoveCorpse.GA_PlayerRemoveCorpse_C" 0 -1)
  (`AbilitySystemComponent.K2_GiveAbility` _abilitysystemcomponent "/Game/Blueprints/AbilitySystem/GameplayAbilities/Player/GA_PlayerRecruitHero.GA_PlayerRecruitHero_C" 0 -1)
  ;[1 1 1] Apply Default Attributes
  (bind _returnvalue (`AbilitySystemBlueprintLibrary.AssignTagSetByCallerMagnitude` (`AbilitySystemComponent.MakeOutgoingSpec` :`self` (`self.AbilitySystemComponent`) :`GameplayEffectClass` "/Game/Blueprints/AbilitySystem/GameplayEffects/Player/GE_SetActionPoints.GE_SetActionPoints_C") (struct :`TagName` "Player.Data.ActionPoints") 2.0))
  (`AbilitySystemComponent.BP_ApplyGameplayEffectSpecToSelf` (`self.AbilitySystemComponent`) _returnvalue)
  (`self.CheckActivePlayer`
    (:`Current`
      (`AbilitySystemComponent.BP_ApplyGameplayEffectToSelf` :`self` (`self.AbilitySystemComponent`) :`GameplayEffectClass` "/Game/Blueprints/AbilitySystem/GameplayEffects/Player/GE_RestoreActionPoints.GE_RestoreActionPoints_C"))
    (:`Not Current`
      _))
  ;[1 1 1] Bind Restoration
  (bind _asbattle_gm (cast `/Game/Blueprints/GameModes/Battle_GM` (`GameplayStatics.GetGameMode`))
    (:`then`
      (bind _output_get (set `self.Battle GM` _asbattle_gm))
      (add `/Game/Blueprints/GameModes/Battle_GM.OnEndTurn` _output_get (`|CreateDelegate` :!event `OnTurnEnd`))
      ;[1 1 1] Bind Apply Damage
      (add `/Game/Blueprints/GameModes/Battle_GM.OnEndWave` (`self.Battle GM`) (`|CreateDelegate` :!event `OnWaveEnd`)))
    (:`CastFailed`
      (`KismetSystemLibrary.PrintString` "Game Mode is not valid(BP_Player)" true true (struct :`R` 1.0 :`A` 1.0)))))

(fn `InitializeCardDescriptionPanel`
  (params (CardDescriptionPanel :type "/Game/Blueprints/Widgets/W_CardDescription Object Reference"))
  (bind _output_get (set `self.CardDescriptionPanel` CardDescriptionPanel))
  (add `/Game/Blueprints/Widgets/W_CardDescription.OnClose` _output_get (`|CreateDelegate` :!event `HideDescriptionPanel`)))

(fn `OnTurnEnd`
  (`self.CheckActivePlayer`
    (:`Current`
      (`AbilitySystemComponent.BP_ApplyGameplayEffectToSelf` :`self` (`self.AbilitySystemComponent`) :`GameplayEffectClass` "/Game/Blueprints/AbilitySystem/GameplayEffects/Player/GE_RestoreActionPoints.GE_RestoreActionPoints_C"))))

(fn `OnWaveEnd`
  (for _array_element (`SquadComponent.GetHeroes` (`self.SquadComponent`))
    (`AbilitySystemComponent.BP_ApplyGameplayEffectToSelf` :`self` (`AbilitySystemBlueprintLibrary.GetAbilitySystemComponent` _array_element) :`GameplayEffectClass` "/Game/Blueprints/AbilitySystem/GameplayEffects/Generic/GE_ApplyDamage.GE_ApplyDamage_C")))

(fn `SetActiveLine`
  (params (IsActive :type Boolean))
  (if IsActive
    (bind _returnvalue (`BattleState.GetLineTurnInt`))
    (bind _returnvalue_2 (`SquadComponent.GetDropZoneInRow` (`self.GetComponentByClass` "/Script/Tactical_Triumph.SquadComponent") _returnvalue))
    (for _array_element _returnvalue_2
      (bind _asbp_drop_zone (cast `/Game/Blueprints/DropZone/BP_DropZone` _array_element))
      (`/Game/Blueprints/DropZone/BP_DropZone.SetActiveMaterial` _asbp_drop_zone true)
      (`KismetArrayLibrary.Array_Add` (`self.ActiveDropZones`) _asbp_drop_zone))
    (else
      (for _array_element_2 (`self.ActiveDropZones`)
        (bind _asbp_drop_zone_2 (cast `/Game/Blueprints/DropZone/BP_DropZone` _array_element_2))
        (`/Game/Blueprints/DropZone/BP_DropZone.SetActiveMaterial` _asbp_drop_zone_2 false))
      (`KismetArrayLibrary.Array_Clear` (`self.ActiveDropZones`)))))

(fn `ShowDescriptionPanel`
  (params (HeroData :type "HeroData Object Reference"))
  (`/Game/Blueprints/Widgets/W_CardDescription.Set Active` (`self.CardDescriptionPanel`) true HeroData false))

(fn `UserConstructionScript`)